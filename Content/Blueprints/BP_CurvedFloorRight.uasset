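; Right-curved floor tile for a runner game, exposing an arrow transform as its attach point.
; One trigger box asks the game mode to extend the floor and raises the player's clamped max walk speed.
; A second box starts turning, after which Tick rotates the player to the spline's rotation near the capsule, interpolating distance between spline points.
; Lane-based obstacle spawning functions exist but are disconnected from the construction script.
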(event OnComponentBeginOverlap(Box)
  (params (OverlappedComponent :type Primitive%20Component%20Object%20Reference) (OtherActor :type Actor%20Object%20Reference) (OtherComp :type Primitive%20Component%20Object%20Reference) (OtherBodyIndex :type Integer) (bFromSweep :type Boolean) (SweepResult :type Hit%20Result%20Structure%20%28by%20ref%29))
  (bind _asbp_player_runner (Utilities|Casting|CastToBP_PlayerRunner OtherActor))
  (Utilities|IsValid (Variables|Default|GetBP_PlayerRunner)
    (:Is%20Valid
      _)
    (:Is%20Not%20Valid
      (Variables|Default|SetBP_PlayerRunner _asbp_player_runner)))
  ;[1 1 1] Extend floor
  (Utilities|IsValid (Variables|Default|GetBP_RunnerGameMode)
    (:Is%20Valid
      (Default|ExtendFloor (Variables|Default|GetBP_RunnerGameMode))
      (Development|PrintString "Floor extended")
      ;[1 1 1] Increase speed
      (bind _output_get (Variables|/Script/Engine.CharacterMovementComponent|SetMaxWalkSpeed (Variables|/Script/Engine.Character|GetCharacterMovement (Variables|Default|GetBP_PlayerRunner)) (Math|Float|Clamp(Float) (* (Variables|/Script/Engine.CharacterMovementComponent|GetMaxWalkSpeed (Variables|/Script/Engine.Character|GetCharacterMovement (Variables|Default|GetBP_PlayerRunner))) 1.02) 7e+02 5e+03)))
      (Development|PrintString (Utilities|String|Append "Max Speed Increased To: " (Utilities|String|ToString(Float) _output_get))))))

(event OnComponentBeginOverlap(Box1)
  (params (OverlappedComponent :type Primitive%20Component%20Object%20Reference) (OtherActor :type Actor%20Object%20Reference) (OtherComp :type Primitive%20Component%20Object%20Reference) (OtherBodyIndex :type Integer) (bFromSweep :type Boolean) (SweepResult :type Hit%20Result%20Structure%20%28by%20ref%29))
  (bind _asbp_player_runner (Utilities|Casting|CastToBP_PlayerRunner OtherActor))
  (Variables|Default|SetTurning true)
  (Variables|/Game/Blueprints/BP_PlayerRunner.BP_PlayerRunner_C|SetTurning _asbp_player_runner true)
  (Default|TurnEvent _asbp_player_runner))

(event EventBeginPlay
  (bind _asbp_runner_game_mode (Utilities|Casting|CastToBP_RunnerGameMode (Game|GetGameMode)))
  (Variables|Default|SetBP_RunnerGameMode _asbp_runner_game_mode)
  (bind _returnvalue (Actor|GetActorOfClass "/Game/Blueprints/BP_PlayerRunner.BP_PlayerRunner_C"))
  (Variables|Default|SetBP_PlayerRunner _returnvalue))

(event Collision|EventActorBeginOverlap
  (params (OtherActor :type Actor%20Object%20Reference)))

(event EventTick
  (params (DeltaSeconds :type Float%20%28single-precision%29))
  (bind _spline (Variables|Default|GetSpline))
  (bind _bp_playerrunner (Variables|Default|GetBP_PlayerRunner))
  (bind _spline_2 (Variables|Default|GetSpline))
  (bind _capsulecomponent (Variables|/Script/Engine.Character|GetCapsuleComponent _bp_playerrunner))
  (bind _returnvalue (Transformation|GetWorldLocation _capsulecomponent))
  (bind _returnvalue_2 (Class|SplineComponent|FindInputKeyClosesttoWorldLocation _spline_2 _returnvalue))
  (bind _returnvalue_3 (Math|Float|Floor _returnvalue_2))
  (bind _returnvalue_4 (+ _returnvalue_3 1))
  (bind _returnvalue_5 (Spline|GetDistanceAlongSplineatSplinePoint _spline _returnvalue_4))
  (if (Variables|Default|GetTurning)
    (Transformation|SetActorRotation (Variables|Default|GetBP_PlayerRunner) (Spline|GetRotationatDistanceAlongSpline (Variables|Default|GetSpline) (- _returnvalue_5 (* (- (Spline|GetDistanceAlongSplineatSplinePoint _spline _returnvalue_3) _returnvalue_5) (- _returnvalue_2 (Math|Conversions|ToFloat(Integer) _returnvalue_4)))) "World"))))

(fn ConstructionScript)

(fn GetAttachPoint
  (return (Transformation|GetWorldTransform (Variables|Default|GetArrow))))

(fn SetupSpawnPoints
  (for _array_element (Variables|Default|GetLanePositions)
    (for _index (range 0 1)
      (bind _returnvalue (AddComponent|AddArrowComponent false (Math|Transform|MakeTransform (Math|Vector|MakeVector (* _index 6.5e+02) _array_element 0.0))))
      (Utilities|Array|Add (Variables|Default|GetSpawnPoints) (Transformation|GetWorldTransform _returnvalue)))))

(fn SpawnObstacles
  (bind _output_get (LocalVariables|SetRandomSpawnPoints (Variables|Default|GetSpawnPoints)))
  (Utilities|Array|Shuffle _output_get)
  (for _index (range 0 (Math|Random|RandomIntegerinRange 0 0))
    (switch int (Math|Random|RandomIntegerinRange 0 1)
      (:0
        (AddComponent|AddChildActorComponent false (Math|Transform|MakeRelativeTransform (Utilities|Array|Get(acopy) (LocalVariables|GetRandomSpawnPoints) _index) (Transformation|GetActorTransform))))
      (:1
        (AddComponent|AddChildActorComponent false (Math|Transform|MakeRelativeTransform (Utilities|Array|Get(acopy) (LocalVariables|GetRandomSpawnPoints) _index) (Transformation|GetActorTransform)))))))