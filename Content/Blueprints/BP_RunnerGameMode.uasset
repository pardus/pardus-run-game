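; BP_RunnerGameMode is a runner game mode that builds the track from chained floor tiles, pre-spawning NumberOfMaxTiles at BeginPlay.
; Each spawned piece supplies the attach point for the next, including right curves, which keep only the latest instance.
; ExtendFloor and the identical ExtendCurvedFloor add straight tiles and trim beyond a five-tile buffer over the maximum.
; Trimming removes index 0 before destroying FloorTiles[0], so the destroy hits the following tile.
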(event EventBeginPlay
  (for _index (range 0 (- (Variables|Default|GetNumberOfMaxTiles) 1))
    (CallFunction|AddFloor)))

(fn ConstructionScript)

(fn AddFloor
  (bind _returnvalue (Game|SpawnActorfromClass "/Game/Blueprints/BP_Floor.BP_Floor_C" (Variables|Default|GetFloorAttachPoint) "Undefined" "MultiplyWithRoot" 0 0))
  (bind _attachtransform (Default|GetAttachPoint _returnvalue))
  (Variables|Default|SetFloorAttachPoint _attachtransform)
  (Utilities|Array|Add (Variables|Default|GetFloorTiles) _returnvalue))

(fn ExtendFloor
  (bind _floortiles (Variables|Default|GetFloorTiles))
  (bind _output (Utilities|Array|Get(acopy) _floortiles))
  (CallFunction|AddFloor)
  (if (> (Utilities|Array|Length (Variables|Default|GetFloorTiles)) (+ (Variables|Default|GetNumberOfMaxTiles) 5))
    (Utilities|Array|RemoveItem _floortiles _output)
    (Actor|DestroyActor _output)))

(fn ExtendCurvedFloor
  (bind _floortiles (Variables|Default|GetFloorTiles))
  (bind _output (Utilities|Array|Get(acopy) _floortiles))
  (CallFunction|AddFloor)
  (if (> (Utilities|Array|Length (Variables|Default|GetFloorTiles)) (+ (Variables|Default|GetNumberOfMaxTiles) 5))
    (Utilities|Array|RemoveItem _floortiles _output)
    (Actor|DestroyActor _output)))

(fn AddCurvedFloorRight
  (Utilities|IsValid (Variables|Default|GetPreviousCurvedFloor)
    (:Is%20Valid
      (Actor|DestroyActor (Variables|Default|GetPreviousCurvedFloor)))
    (:Is%20Not%20Valid
      _))
  (bind _returnvalue (Game|SpawnActorfromClass "/Game/Blueprints/BP_CurvedFloorRight.BP_CurvedFloorRight_C" (Variables|Default|GetFloorAttachPoint) "Undefined" "MultiplyWithRoot" 0 0))
  (bind _output_get (Variables|Default|SetPreviousCurvedFloor _returnvalue))
  (bind _attachtransform (Default|GetAttachPoint _output_get))
  (Variables|Default|SetFloorAttachPoint _attachtransform))