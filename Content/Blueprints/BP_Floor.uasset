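; Floor tile for an endless runner with lane obstacles and randomised motherboard-themed scenery.
; Construction builds lane spawn points, places one child-actor obstacle at a shuffled point and randomly toggles or moves decor.
; Box overlap by the runner calls the game mode's ExtendFloor, then raises capped walk speed and scales animation rate to match.
; GetAttachPoint exposes the arrow transform; curved-floor and sine-bobbing logic is unwired.
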(event OnComponentBeginOverlap(Box)
  (params (OverlappedComponent :type Primitive%20Component%20Object%20Reference) (OtherActor :type Actor%20Object%20Reference) (OtherComp :type Primitive%20Component%20Object%20Reference) (OtherBodyIndex :type Integer) (bFromSweep :type Boolean) (SweepResult :type Hit%20Result%20Structure%20%28by%20ref%29))
  (bind _asbp_player_runner (Utilities|Casting|CastToBP_PlayerRunner OtherActor))
  (Utilities|IsValid (Variables|Default|GetBP_PlayerRunner)
    (:Is%20Valid
      _)
    (:Is%20Not%20Valid
      (Variables|Default|SetBP_PlayerRunner _asbp_player_runner)))
  ;[1 1 1] Extend floor
  (Utilities|IsValid (Variables|Default|GetBP_RunnerGameMode)
    (:Is%20Valid
      (Default|ExtendFloor (Variables|Default|GetBP_RunnerGameMode))
      (Development|PrintString "Floor extended")
      ;[1 1 1] Increase speed
      (Variables|/Script/Engine.SkeletalMeshComponent|SetGlobalAnimRateScale (Variables|/Script/Engine.Character|GetMesh (Variables|Default|GetBP_PlayerRunner)) (Math|Float|MapRangeUnclamped (* (Variables|/Script/Engine.CharacterMovementComponent|GetMaxWalkSpeed (Variables|/Script/Engine.Character|GetCharacterMovement (Variables|Default|GetBP_PlayerRunner))) 1.006) 1.8e+03 1e+04 1.0 5.0))
      (bind _output_get (Variables|/Script/Engine.CharacterMovementComponent|SetMaxWalkSpeed (Variables|/Script/Engine.Character|GetCharacterMovement (Variables|Default|GetBP_PlayerRunner)) (Math|Float|Clamp(Float) (* (Variables|/Script/Engine.CharacterMovementComponent|GetMaxWalkSpeed (Variables|/Script/Engine.Character|GetCharacterMovement (Variables|Default|GetBP_PlayerRunner))) 1.006) 1.8e+03 1e+04)))
      (Development|PrintString (Utilities|String|Append "Max Speed Extended To: " (Utilities|String|ToString(Float) _output_get))))))

(event Custom|Move
  (params (Speed :type Float%20%28double-precision%29) (Target2 :type Scene%20Component%20Object%20Reference))
  (Transformation|AddLocalOffset Target2 (Math|Vector|MakeVector 0.0 0.0 (* (Math|Trig|Sin(Radians) (* Speed (Utilities|Time|GetGameTimeinSeconds))) (Variables|Default|GetRange))) false false))

(event EventBeginPlay
  (bind _asbp_runner_game_mode (Utilities|Casting|CastToBP_RunnerGameMode (Game|GetGameMode)))
  (Variables|Default|SetBP_RunnerGameMode _asbp_runner_game_mode)
  (bind _returnvalue (Actor|GetActorOfClass "/Game/Blueprints/BP_PlayerRunner.BP_PlayerRunner_C"))
  (Variables|Default|SetBP_PlayerRunner _returnvalue))

(event Collision|EventActorBeginOverlap
  (params (OtherActor :type Actor%20Object%20Reference)))

(event EventTick
  (params (DeltaSeconds :type Float%20%28single-precision%29)))

(fn ConstructionScript
  (CallFunction|SetupSpawnPoints)
  (CallFunction|SpawnObstacles)
  (CallFunction|SpawnEnvironment))

(fn GetAttachPoint
  (return (Transformation|GetWorldTransform (Variables|Default|GetArrow))))

(fn SetupSpawnPoints
  (for _array_element (Variables|Default|GetLanePositions)
    (for _index (range 0 1)
      (bind _returnvalue (AddComponent|AddArrowComponent false (Math|Transform|MakeTransform (Math|Vector|MakeVector (* _index 6.5e+02) _array_element 0.0))))
      (Utilities|Array|Add (Variables|Default|GetSpawnPoints) (Transformation|GetWorldTransform _returnvalue)))))

(fn SpawnObstacles
  (bind _output_get (LocalVariables|SetRandomSpawnPoints (Variables|Default|GetSpawnPoints)))
  (Utilities|Array|Shuffle _output_get)
  (for _index (range 0 (Math|Random|RandomIntegerinRange 0 0))
    (switch int (Math|Random|RandomIntegerinRange 1 2)
      (:0
        (AddComponent|AddChildActorComponent false (Math|Transform|MakeRelativeTransform (Utilities|Array|Get(acopy) (LocalVariables|GetRandomSpawnPoints) _index) (Transformation|GetActorTransform))))
      (:1
        (AddComponent|AddChildActorComponent false (Math|Transform|MakeRelativeTransform (Utilities|Array|Get(acopy) (LocalVariables|GetRandomSpawnPoints) _index) (Transformation|GetActorTransform))))
      (:2
        (AddComponent|AddChildActorComponent false (Math|Transform|MakeRelativeTransform (Utilities|Array|Get(acopy) (LocalVariables|GetRandomSpawnPoints) _index) (Transformation|GetActorTransform)))))))

(fn SpawnEnvironment
  (if (Math|Random|RandomBoolwithWeight 0.7)
    (Rendering|SetVisibility (Variables|Default|GetPardusMotherboards_pCube29) false true))
  (if (Math|Random|RandomBoolwithWeight 0.7)
    (Rendering|SetVisibility (Variables|Default|GetPardusMotherboards_pCylinder68) false true))
  (if (Math|Random|RandomBoolwithWeight 0.7)
    (Rendering|SetVisibility (Variables|Default|GetPardusMotherboards_pCylinder67) false true))
  (if (Math|Random|RandomBoolwithWeight 0.7)
    (Rendering|SetVisibility (Variables|Default|GetPardusMotherboards_pCylinder4) false true))
  (if (Math|Random|RandomBoolwithWeight 0.7)
    (Rendering|SetVisibility (Variables|Default|GetPardusMotherboards_pCube1) false true))
  (if (Math|Random|RandomBoolwithWeight 0.7)
    (Rendering|SetVisibility (Variables|Default|GetPardusMotherboards_pCylinder71) false true))
  (if (Math|Random|RandomBoolwithWeight 0.7)
    (Rendering|SetVisibility (Variables|Default|GetPardusMotherboards_pCylinder70) false true))
  (if (Math|Random|RandomBoolwithWeight 0.7)
    _
    (else
      _))
  (Rendering|SetVisibility (Variables|Default|GetPardusMotherboards_pCylinder69) false true)
  (if (Math|Random|RandomBoolwithWeight 0.9)
    (Rendering|SetVisibility (Variables|Default|GetPardusMotherboards_pCube38) false true))
  (if (Math|Random|RandomBoolwithWeight 0.7)
    (Rendering|SetVisibility (Variables|Default|GetPardusMotherboards_pCube32) false true))
  (if (Math|Random|RandomBoolwithWeight 0.7)
    (Rendering|SetVisibility (Variables|Default|GetPardusMotherboards_pCube33) false true))
  (if (Math|Random|RandomBoolwithWeight 0.7)
    _
    (else
      _))
  (Rendering|SetVisibility (Variables|Default|GetPardusMotherboards_pCylinder74) false true)
  (if (Math|Random|RandomBoolwithWeight 0.8)
    (Rendering|SetVisibility (Variables|Default|GetBP_GPU_1) false true)
    (elif (Math|Random|RandomBoolwithWeight 0.5)
      (Transformation|SetRelativeLocation (Variables|Default|GetBP_GPU_1) "980.000000,1504.000000,-199.999971" false false)
      (Transformation|AddRelativeLocation (Variables|Default|GetPardusMotherboards_pCube73) "0.000000,-32600.000000,0.000000" false false)))
  (if (Math|Random|RandomBoolwithWeight 0.1)
    (Rendering|SetVisibility (Components|GetChildComponent (Variables|Default|GetSolKartlar) (Math|Random|RandomIntegerinRange 0 4)) true false))
  (if (Math|Random|RandomBoolwithWeight 0.1)
    (Rendering|SetVisibility (Components|GetChildComponent (Variables|Default|GetSagKartlar) (Math|Random|RandomIntegerinRange 0 4)) true false)))