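; BP_Collectable is a coin pickup that the BP_PlayerRunner character collects by overlapping it.
; A fast looping timer spins the coin mesh through small relative rotations instead of using Tick.
; On overlap with the runner it calls the runner's Collect, plays a coin sound, hides itself and destroys itself after a short delay.
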(event Custom|Rotate
  (Transformation|AddRelativeRotation (Variables|Default|GetPardusCoin_PardusCoin) "0.000000,3.000000,0.000000" false false))

(event EventBeginPlay
  (Utilities|Time|SetTimerbyEvent (delegate Custom|Rotate) 0.01 true))

(event Collision|EventActorBeginOverlap
  (params (OtherActor :type Actor%20Object%20Reference))
  (bind _asbp_player_runner (Utilities|Casting|CastToBP_PlayerRunner OtherActor))
  (Default|Collect _asbp_player_runner)
  (Audio|PlaySound2D "/Game/Sounds/Coin.Coin" 1.0 1.0 0.0 0 0)
  (Rendering|SetActorHiddenInGame true)
  (Utilities|FlowControl|Delay 1.0)
  (Actor|DestroyActor))

(event EventTick
  (params (DeltaSeconds :type Float%20%28single-precision%29)))

(fn ConstructionScript)